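; Player-controllable tank Blueprint that drives on two tracks, orbits an aiming camera and fires projectiles.
; Construction assigns turret, barrel and track meshes plus a track friction material, and BeginPlay registers the barrel and turret references.
; Throttle axes drive each track directly, while a joystick axis sends forward intent to TankMovementComponent.
; Aim axes yaw an azimuth gimbal and pitch the spring arm separately, and the fire action calls Fire.
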(event EventBeginPlay
  (Class|Tank|SetBarrelReference (Variables|Default|GetBarrel))
  (Class|Tank|SetTurretReference (Variables|Default|GetTurret)))

(event Input|ActionEvents|InputActionFireProjectile
  (params (Key :type Key%20Structure))
  ;[1 1 1] Aiming Input Bindings
  (:Pressed
    (Class|Tank|Fire)))

(event Input|AxisEvents|InputAxisAimAzimuth
  (params (AxisValue :type Float%20%28single-precision%29))
  ;[1 1 1] Aiming Input Bindings
  (Transformation|AddLocalRotation (Variables|Default|GetAzimuth%20Gimbal) (Math|Rotator|MakeRotator 0.0 0.0 AxisValue) false false))

(event Input|AxisEvents|InputAxisAimElevation
  (params (AxisValue :type Float%20%28single-precision%29))
  ;[1 1 1] Aiming Input Bindings
  (Transformation|AddLocalRotation (Variables|Default|GetSpringArm) (Math|Rotator|MakeRotator 0.0 AxisValue 0.0) false false))

(event Input|AxisEvents|InputAxisLeftTrackThrottle
  (params (AxisValue :type Float%20%28single-precision%29))
  ;[1 1 1] Movement Input Bindings
  (Class|TankTrack|SetThrottle (Variables|Default|GetLeftTrack) AxisValue))

(event Input|AxisEvents|InputAxisRightTrackThrottle
  (params (AxisValue :type Float%20%28single-precision%29))
  ;[1 1 1] Movement Input Bindings
  (Class|TankTrack|SetThrottle (Variables|Default|GetRightTrack) AxisValue))

(event Input|AxisEvents|InputAxisJoyStickMovement
  (params (AxisValue :type Float%20%28single-precision%29))
  ;[1 1 1] Movement Input Bindings
  (Class|TankMovementComponent|IntendMoveForward (Variables|Default|GetTankMovementComponent) AxisValue))

(fn ConstructionScript
  (Components|StaticMesh|SetStaticMesh (Variables|Default|GetTurret) "/Game/TankFolder/tank_fbx_Turret.tank_fbx_Turret")
  (Components|StaticMesh|SetStaticMesh (Variables|Default|GetBarrel) "/Game/TankFolder/tank_fbx_Barrel.tank_fbx_Barrel")
  (Components|StaticMesh|SetStaticMesh (Variables|Default|GetLeftTrack) "/Game/TankFolder/tank_fbx_Track.tank_fbx_Track")
  (Class|PrimitiveComponent|SetPhysMaterialOverride (Variables|Default|GetLeftTrack) "/Game/TankFolder/TrackFriction.TrackFriction")
  (Components|StaticMesh|SetStaticMesh (Variables|Default|GetRightTrack) "/Game/TankFolder/tank_fbx_Track.tank_fbx_Track")
  (Class|PrimitiveComponent|SetPhysMaterialOverride (Variables|Default|GetRightTrack) "/Game/TankFolder/TrackFriction.TrackFriction"))